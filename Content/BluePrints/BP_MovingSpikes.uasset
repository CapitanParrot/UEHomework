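; BP_MovingSpikes is a legacy spike trap, marked as superseded by sphereSpikes, that moves a child actor along a spline.
; Init loads stats from DT_MovingSpikes and registers with BP_GM, then a timeline drives movement.
; SpeedUp and SpeedDown rescale the timeline's play rate.
; While the player overlaps, a fast looping timer applies damage and outward impulse unless the GameMode flags IsRockHard or IsInvincible.
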(event EventBeginPlay
  ;[1 0 0.1205] Стараяя ловушка, не оправдала ожиданий, лучше используйте sphereSpikes
  (Utilities|Init
    (:Out
      (Components|Timeline|SetPlayRate (Variables|Default|GetMovingTime) (.speed (Variables|Default|GetSpikeStats)))
      (bind _time (Timeline|MovingTime Play)
        (:Update
          (Transformation|SetWorldLocation (Variables|Default|GetChildActor) (Spline|GetLocationatTime (Variables|Default|GetSpline) _time "World" false) false false))))))

(event Collision|EventActorEndOverlap
  (params (OtherActor :type Actor%20Object%20Reference))
  ;[1 0 0.1205] Стараяя ловушка, не оправдала ожиданий, лучше используйте sphereSpikes
  (Utilities|Casting|CastToBP_ThirdPersonCharacter OtherActor)
  (Utilities|Time|ClearTimerbyFunctionName 0 "OnSpikes"))

(event EventSpeedUp
  (params (Amount :type Float%20%28double-precision%29))
  ;[1 0 0.1205] Стараяя ловушка, не оправдала ожиданий, лучше используйте sphereSpikes
  ;;[1 1 1] Увеличение скорости у ловушки
  (Development|PrintString (Utilities|String|ToString(Float) Amount) true true "(R=0.010857,G=1.000000,B=0.162320,A=1.000000)")
  (bind _output_get (Variables|Default|SetSpikeStats (Utilities|Struct|MakeS_MovingSpikes (.damage (Variables|Default|GetSpikeStats)) (.pushforce (Variables|Default|GetSpikeStats)) (* Amount (.speed (Variables|Default|GetSpikeStats))))))
  (Development|PrintString (Utilities|String|ToString(Float) (.speed _output_get)) true true "(R=0.660202,G=1.000000,B=0.000000,A=1.000000)")
  (Components|Timeline|SetPlayRate (Variables|Default|GetMovingTime) (.speed _output_get)))

(event EventSpeedDown
  (params (Amount :type Float%20%28double-precision%29))
  ;[1 0 0.1205] Стараяя ловушка, не оправдала ожиданий, лучше используйте sphereSpikes
  ;;[1 1 1] Уменьшение скорости у ловушки
  (bind _output_get (Variables|Default|SetSpikeStats (Utilities|Struct|MakeS_MovingSpikes (.damage (Variables|Default|GetSpikeStats)) (.pushforce (Variables|Default|GetSpikeStats)) (/ (.speed (Variables|Default|GetSpikeStats)) Amount))))
  (Development|PrintString (Utilities|String|ToString(Float) (.speed _output_get)) true true "(R=1.000000,G=0.123137,B=0.250957,A=1.000000)")
  (Components|Timeline|SetPlayRate (Variables|Default|GetMovingTime) (.speed _output_get)))

(event Collision|EventActorBeginOverlap
  (params (OtherActor :type Actor%20Object%20Reference))
  ;[1 0 0.1205] Стараяя ловушка, не оправдала ожиданий, лучше используйте sphereSpikes
  ;;[1 1 1] Обработка столкновения с игроком
  (bind _asbp_third_person_character (Utilities|Casting|CastToBP_ThirdPersonCharacter OtherActor))
  (Variables|Default|SetPlayer _asbp_third_person_character)
  (Utilities|Time|SetTimerbyFunctionName 0 "OnSpikes" 0.01 true))

(fn ConstructionScript)

(fn Push
  (bind _returnvalue (Transformation|GetActorTransform))
  (bind _player (Variables|Default|GetPlayer))
  (bind _spikestats (Variables|Default|GetSpikeStats))
  (bind _returnvalue_2 (Transformation|GetActorLocation _player))
  (bind _returnvalue_3 (- _returnvalue_2 (.location _returnvalue)))
  (bind _returnvalue_4 (Math|Vector|Normalize _returnvalue_3))
  (bind _returnvalue_5 (* _returnvalue_4 (.pushforce _spikestats)))
  (Development|PrintString (Utilities|String|ToString(Vector) _returnvalue_5))
  (Physics|AddImpulse (Variables|/Script/Engine.Character|GetCharacterMovement (Variables|Default|GetPlayer)) _returnvalue_5 true))

(fn OnSpikes
  (bind _gamemode (Variables|Default|GetGameMode))
  (if (not (Variables|/Game/BluePrints/BP_GM.BP_GM_C|GetIsRockHard _gamemode))
    (if (not (Variables|/Game/BluePrints/BP_GM.BP_GM_C|GetIsInvincible _gamemode))
      (Default|TakeDamage _gamemode (.damage (Variables|Default|GetSpikeStats)))
      (CallFunction|Push))))