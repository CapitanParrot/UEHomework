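; BP_Spikes is a static spike hazard that damages and knocks back the third-person character while it overlaps the actor.
; On BeginPlay it caches BP_GM and loads its stats from the DT_StaticSpikes data table.
; Overlap starts a fast looping timer, cleared on exit, that applies damage through the game mode unless the player is rock-hard, invincible or dead.
; Each hit also launches the player away from the spikes with a velocity-change impulse.
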(event EventBeginPlay
  (Utilities|InitSpikes))

(event Collision|EventActorEndOverlap
  (params (OtherActor :type Actor%20Object%20Reference))
  (Utilities|Casting|CastToBP_ThirdPersonCharacter OtherActor)
  (Utilities|Time|ClearTimerbyFunctionName 0 "OnSpikes"))

(event Collision|EventActorBeginOverlap
  (params (OtherActor :type Actor%20Object%20Reference))
  (bind _asbp_third_person_character (Utilities|Casting|CastToBP_ThirdPersonCharacter OtherActor))
  (Variables|Default|SetPlayer _asbp_third_person_character)
  (Utilities|Time|SetTimerbyFunctionName 0 "OnSpikes" 0.009 true))

(fn ConstructionScript)

(fn Push
  (bind _returnvalue (Transformation|GetActorTransform))
  (bind _spikesstats (Variables|Default|GetSpikesStats))
  (bind _player (Variables|Default|GetPlayer))
  (bind _returnvalue_2 (Transformation|GetActorLocation _player))
  (bind _returnvalue_3 (- _returnvalue_2 (.location _returnvalue)))
  (bind _returnvalue_4 (Math|Vector|Normalize _returnvalue_3))
  (bind _returnvalue_5 (* _returnvalue_4 (.pushforce _spikesstats)))
  (Development|PrintString (Utilities|String|ToString(Vector) _returnvalue_5))
  (Physics|AddImpulse (Variables|/Script/Engine.Character|GetCharacterMovement (Variables|Default|GetPlayer)) _returnvalue_5 true))

(fn OnSpikes
  (bind _gamemode (Variables|Default|GetGameMode))
  (if (not (Math|Boolean|ORBoolean (Variables|/Game/BluePrints/BP_GM.BP_GM_C|GetIsRockHard _gamemode) (Variables|/Game/BluePrints/BP_GM.BP_GM_C|GetIsInvincible _gamemode) (Variables|/Game/BluePrints/BP_GM.BP_GM_C|GetIsPlayerDead _gamemode)))
    (Default|TakeDamage (Variables|Default|GetGameMode) (.damage (Variables|Default|GetSpikesStats)))
    (CallFunction|Push)))