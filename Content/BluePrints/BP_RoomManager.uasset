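; Room manager that populates a room with random acts and places the player at its entrance.
; On BeginPlay it registers itself as the game mode's current room, then spawns an act at each hand-assigned spawn point.
; Each act is a random row from the hard or easy data table, chosen by IsHard.
; It then teleports the player beside the entrance door and clears the dead flag as a damage workaround.
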(event Custom|AddSpawnPoint
  (params (Point :type BP%20Act%20Spwan%20Point%20Object%20Reference))
  ;[1 0 0.08432] Добавляет точку спавна в массив. Не используется потому что точки добавлялись раньше чем инициализируется RoomManager, Теперь добавляем точки руками в массив
  (Utilities|Array|Add (Variables|Default|GetSpawnPoints) Point)
  (if (== (Utilities|Array|Length (Variables|Default|GetSpawnPoints)) (Variables|Default|GetPointsMax))
    _))

(event Custom|SpawnActs
  ;[1 1 1] Спавнит акты на местах точек спавна
  (bind _result (Math|Integer|DecrementInt (Utilities|Array|Length (Variables|Default|GetSpawnPoints)))
    (:%20%20
      (for _index (range 0 _result)
        (bind _act (CallFunction|GetAct))
        (Game|SpawnActorfromClass _act (Math|Transform|MakeTransform (.location (Transformation|GetActorTransform (Utilities|Array|Get(acopy) (Variables|Default|GetSpawnPoints) _index))) (.rotation (Transformation|GetActorTransform (Utilities|Array|Get(acopy) (Variables|Default|GetSpawnPoints) _index))) "1.000000,1.000000,1.000000") "Undefined" 0 0)))))

(event Custom|TeleportPlayer
  ;[1 1 1] Телепортирует игрока ко входной двери
  (Transformation|Teleport (Variables|/Game/BluePrints/BP_GM.BP_GM_C|GetPlayer (Variables|Default|GetGameMode)) (+ (.location (Transformation|GetActorTransform (Variables|Default|GetEnterDoor))) "0.000000,100.000000,0") "0, 0, 0")
  ;;[0.003805 1 0.03141] Костыльный костыль, Чтобы персонаж не получал урон до перезапуска
  (if (Variables|/Game/BluePrints/BP_GM.BP_GM_C|GetIsPlayerDead (Variables|Default|GetGameMode))
    (Variables|/Game/BluePrints/BP_GM.BP_GM_C|SetIsPlayerDead (Variables|Default|GetGameMode) false)))

(event EventBeginPlay
  (bind _asbp_gm (Utilities|Casting|CastToBP_GM (Game|GetGameMode)))
  (bind _output_get (Variables|Default|SetGameMode _asbp_gm))
  (Variables|/Game/BluePrints/BP_GM.BP_GM_C|SetCurrentRoom _output_get self)
  (CallFunction|SpawnActs)
  (CallFunction|TeleportPlayer))

(fn ConstructionScript)

(fn GetAct
  ;[1 1 1] Выдает случайный акт в зависимости от сложности комнаты
  (if (Variables|Default|GetIsHard)
    (bind _outrownames (DataTable|GetDataTableRowNames "/Game/DataTables/DT_HardActs.DT_HardActs"))
    (bind _returnvalue (Utilities|GetDataTableRow "/Game/DataTables/DT_HardActs.DT_HardActs" (Utilities|Array|Get(acopy) _outrownames (Math|Random|RandomInteger (Utilities|Array|Length _outrownames))))
      (:then
        (return (.act _returnvalue))))
    (else
      (bind _outrownames_2 (DataTable|GetDataTableRowNames "/Game/DataTables/DT_EasyActs.DT_EasyActs"))
      (bind _returnvalue_2 (Utilities|GetDataTableRow "/Game/DataTables/DT_EasyActs.DT_EasyActs" (Utilities|Array|Get(acopy) _outrownames_2 (Math|Random|RandomInteger (Utilities|Array|Length _outrownames_2))))
        (:then
          (return (.act _returnvalue_2)))))))