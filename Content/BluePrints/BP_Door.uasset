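; BP_Door is a door actor that detects when the player character comes near it.
; On overlap it sets the character's IsNearDoor flag and passes itself as the Door reference; leaving clears only the flag.
; Doors marked IsExit also toggle a Press E prompt through the HealthWidget held by BP_GM, which is cached on BeginPlay.
; The door holds no opening or interaction logic itself.
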(event EventBeginPlay
  (bind _asbp_gm (Utilities|Casting|CastToBP_GM (Game|GetGameMode)))
  (Variables|Default|SetGameMode _asbp_gm))

(event Collision|EventActorBeginOverlap
  (params (OtherActor :type Actor%20Object%20Reference))
  ;[1 1 1] Игрок подешел к двери
  (bind _asbp_third_person_character (Utilities|Casting|CastToBP_ThirdPersonCharacter OtherActor))
  (Variables|/Game/ThirdPerson/Blueprints/BP_ThirdPersonCharacter.BP_ThirdPersonCharacter_C|SetIsNearDoor _asbp_third_person_character true)
  (Variables|/Game/ThirdPerson/Blueprints/BP_ThirdPersonCharacter.BP_ThirdPersonCharacter_C|SetDoor _asbp_third_person_character self)
  (if (Variables|Default|GetIsExit)
    (Default|OnPressE (Variables|/Game/BluePrints/BP_GM.BP_GM_C|GetHealthWidget (Variables|Default|GetGameMode)))))

(event Collision|EventActorEndOverlap
  (params (OtherActor :type Actor%20Object%20Reference))
  ;[1 1 1] Игрок отошел от двери
  (bind _asbp_third_person_character (Utilities|Casting|CastToBP_ThirdPersonCharacter OtherActor))
  (Variables|/Game/ThirdPerson/Blueprints/BP_ThirdPersonCharacter.BP_ThirdPersonCharacter_C|SetIsNearDoor _asbp_third_person_character false)
  (if (Variables|Default|GetIsExit)
    (Default|OffPressE (Variables|/Game/BluePrints/BP_GM.BP_GM_C|GetHealthWidget (Variables|Default|GetGameMode)))))

(fn ConstructionScript)