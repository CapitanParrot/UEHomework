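; BP_Potion is a pickup that randomly becomes a good, neutral or bad potion, or a fixed heal potion when flagged.
; On BeginPlay it picks a group using the BP_GM chances for the room's difficulty.
; It then rolls against each table entry's threshold until one passes, applying that mesh and liquid material.
; Player overlap calls the GameMode effect matching group and ID, then destroys the potion.
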(event Custom|SetupPotion
  (bind _returnvalue (Math|Random|RandomInteger 100))
  (bind _gamemode (Variables|Default|GetGameMode))
  (bind _staticmesh (Variables|Default|GetStaticMesh))
  (bind _staticmesh_2 (Variables|Default|GetStaticMesh))
  (bind _staticmesh_3 (Variables|Default|GetStaticMesh))
  ;[1 1 1] Зелье самостоятельно выбирает кем стать исхлдя из типа комнаты и шансов выпадения зелий
  (if (Variables|Default|GetIsHealPotion)
    (Variables|Default|SetPotionGroupMarker 0)
    ;[1 1 1] Зелье лечения особенное и его можно выставить руками в сложных комантах
    (bind _returnvalue_2 (Utilities|GetDataTableRow "/Game/DataTables/DT_GoodPotions.DT_GoodPotions" "HealPotion")
      (:then
        (bind _output_get (Variables|Default|SetPotion _returnvalue_2))
        (Components|StaticMesh|SetStaticMesh (Variables|Default|GetStaticMesh) (.staticmesh _output_get))))
    (else
      (if (Variables|/Game/BluePrints/BP_RoomManager.BP_RoomManager_C|GetIsHard (Variables|/Game/BluePrints/BP_GM.BP_GM_C|GetCurrentRoom (Variables|Default|GetGameMode)))
        (Variables|Default|SetCurrentChances (Variables|/Game/BluePrints/BP_GM.BP_GM_C|GetHardChance _gamemode))
        (else
          (Variables|Default|SetCurrentChances (Variables|/Game/BluePrints/BP_GM.BP_GM_C|GetEasyChance _gamemode))))
      (if (< _returnvalue (.goodpotions (Variables|Default|GetCurrentChances)))
        (Variables|Default|SetPotionGroupMarker 0)
        ;[1 1 1] Выдает хорошее зелье
        (bind _array_element (Utilities|Array|ForEachLoopwithBreak (Variables|/Game/BluePrints/BP_GM.BP_GM_C|GetGoodPotions (Variables|Default|GetGameMode)) :!label _label)
          (:LoopBody
            (if (< (Math|Random|RandomInteger 100) (.chance _array_element))
              (bind _output_get_2 (Variables|Default|SetPotion (Utilities|Struct|MakeS_Potion (.id _array_element) (.name _array_element) (.description _array_element) (.duration _array_element) (.quantityeffect _array_element) (.chance _array_element) (.staticmesh _array_element) (.material _array_element))))
              (Components|StaticMesh|SetStaticMesh _staticmesh_3 (.staticmesh _output_get_2))
              (Rendering|Material|SetMaterial _staticmesh_3 1 (.material _output_get_2)) ; В ассете potion3 материал жидкости с индексом 1
              (goto _label Break))))
        (elif (< _returnvalue (.neutralpotions (Variables|Default|GetCurrentChances)))
          ;[1 1 1] Выдает нейтральное зелье
          (Variables|Default|SetPotionGroupMarker 1)
          (bind _array_element_2 (Utilities|Array|ForEachLoopwithBreak (Variables|/Game/BluePrints/BP_GM.BP_GM_C|GetNeutralPotions (Variables|Default|GetGameMode)) :!label _label_2)
            (:LoopBody
              (if (< (Math|Random|RandomInteger 100) (.chance _array_element_2))
                (bind _output_get_3 (Variables|Default|SetPotion (Utilities|Struct|MakeS_Potion (.id _array_element_2) (.name _array_element_2) (.description _array_element_2) (.duration _array_element_2) (.quantityeffect _array_element_2) (.chance _array_element_2) (.staticmesh _array_element_2) (.material _array_element_2))))
                (Components|StaticMesh|SetStaticMesh _staticmesh_2 (.staticmesh _output_get_3))
                (Rendering|Material|SetMaterial _staticmesh_2 1 (.material _output_get_3)) ; В ассете potion3 материал жидкости с индексом 1
                (goto _label_2 Break))))
          (else
            ;[1 1 1] Выдает плохое зелье
            (Variables|Default|SetPotionGroupMarker 2)
            (bind _array_element_3 (Utilities|Array|ForEachLoopwithBreak (Variables|/Game/BluePrints/BP_GM.BP_GM_C|GetBadPotions (Variables|Default|GetGameMode)) :!label _label_3)
              (:LoopBody
                (if (< (Math|Random|RandomInteger 100) (.chance _array_element_3))
                  (bind _output_get_4 (Variables|Default|SetPotion (Utilities|Struct|MakeS_Potion (.id _array_element_3) (.name _array_element_3) (.description _array_element_3) (.duration _array_element_3) (.quantityeffect _array_element_3) (.chance _array_element_3) (.staticmesh _array_element_3) (.material _array_element_3))))
                  (Components|StaticMesh|SetStaticMesh _staticmesh (.staticmesh _output_get_4))
                  (Rendering|Material|SetMaterial _staticmesh 1 (.material _output_get_4)) ; В ассете potion3 материал жидкости с индексом 1
                  (goto _label_3 Break))))))))))

(event EventBeginPlay
  (bind _asbp_gm (Utilities|Casting|CastToBP_GM (Game|GetGameMode)))
  (Variables|Default|SetGameMode _asbp_gm)
  (CallFunction|SetupPotion))

(event Collision|EventActorBeginOverlap
  (params (OtherActor :type Actor%20Object%20Reference))
  (bind _gamemode (Variables|Default|GetGameMode))
  (bind _potion (Variables|Default|GetPotion))
  ;[1 1 1] Выбор эффекта зелья при соприкасновении с игроком
  (Utilities|Casting|CastToBP_ThirdPersonCharacter OtherActor)
  (switch int (Variables|Default|GetPotionGroupMarker)
    (:0
      (switch int (.id _potion)
        (:0
          (Default|HealPotion _gamemode)
          (Development|PrintString "Heal"))
        (:1
          (Default|TimePotion _gamemode)
          (Development|PrintString "Time"))
        (:2
          (Default|RockPotion _gamemode)
          (Development|PrintString "Rock"))))
    (:1
      (switch int (.id _potion)
        (:0
          (Default|RandomPotion _gamemode)
          (Development|PrintString "Random"))
        (:1
          (Default|NothingPotion _gamemode)
          (Development|PrintString "Nothing"))))
    (:2
      (switch int (.id _potion)
        (:0
          (Default|SlowPotion _gamemode)
          (Development|PrintString "Slow"))
        (:1
          (Default|PainPotion _gamemode)
          (Development|PrintString "Pain")))))
  (Actor|DestroyActor))

(fn ConstructionScript)